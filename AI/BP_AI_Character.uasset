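; Enemy AI character that roams or patrols, then chases a seen first-person player and explodes on arrival, dealing damage and destroying itself.
; AIState selects the starting behavior: random navmesh roaming, chasing, or patrol between three target points with random waits and branches.
; PawnSensing triggers the chase, and a failed chase falls back to patrol.
; The player's death event disables sensing updates, which gate chasing, and reapplies the AIState behavior.
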(event OnSeePawn(PawnSensing)
  (params (Pawn :type Pawn%20Object%20Reference))
  ;[1 1 1] Chase player when seen
  (bind _asfirst_person_character (Utilities|Casting|CastToFirstPersonCharacter Pawn))
  (CallFunction|ChasePlayer _asfirst_person_character))

(event Custom|MoveToRandomLocation
  ;[1 1 1] Roam
  (AI|AIMoveTo self (.RandomLocation (Class|NavigationSystemV1|GetRandomPointinNavigableRadius (Transformation|GetActorLocation) 5e+02 0 0)) 0 5.0 false :!label _label
    (:OnSuccess
      (Utilities|FlowControl|Delay (Math|Random|RandomFloatinRange 1.0 5.0))
      (goto _label))))

(event Custom|Chase_Player
  (params (PlayerToChase :type Pawn%20Object%20Reference))
  (bind _returnvalue (Transformation|GetActorLocation))
  (bind _self self)
  ;[1 1 1] Fixes bug for pawn sensing, makes it go back to not chasing
  (if (Variables|/Script/AIModule.PawnSensingComponent|GetbEnableSensingUpdates (Variables|Default|GetPawnSensing))
    ;[1 1 1] Chase player
    (AI|AIMoveTo _self "0, 0, 0" PlayerToChase 5.0 false
      (:OnSuccess
        (Game|Damage|ApplyDamage PlayerToChase (Variables|Default|GetDamage) 0 0)
        (Effects|SpawnEmitteratLocation "/Game/StarterContent/Particles/P_Explosion.P_Explosion" _returnvalue)
        (Audio|PlaySoundatLocation "/Game/StarterContent/Audio/Explosion_Cue.Explosion_Cue" _returnvalue "0, 0, 0" 1.0 1.0 0.0 0 0 0)
        (Actor|DestroyActor))
      (:OnFail
        (Utilities|FlowControl|Delay 1.0)
        (CallFunction|Patrol _self)))))

(event Custom|Patrol
  ;[1 1 1] Patrol
  ;;[1 1 1] Target 1
  (AI|AIMoveTo self "0, 0, 0" (Variables|Default|GetTargetPoint1) 5.0 false :!label _label
    (:OnSuccess
      (Utilities|FlowControl|Delay (Math|Random|RandomFloatinRange 2.0 5.0))
      (CallFunction|Patrol)
      ;;[1 0.5052 0.5052] I rng = 0 move to 2, if 1 move to 3
      (if (== (Variables|Default|Get0) (Math|Random|RandomIntegerinRange 0 1))
        ;;[1 1 1] TARGET 2
        (AI|AIMoveTo self "0, 0, 0" (Variables|Default|GetTargetPoint2) 5.0 false :!label _label_2
          (:OnSuccess
            (Utilities|FlowControl|Delay (Math|Random|RandomFloatinRange 1.0 4.0))
            (CallFunction|Patrol)
            ;;[1 0.3958 0.4262] If rng = 0 move to target 3, if = 1 move to target 1
            (if (== (Variables|Default|Get0) (Math|Random|RandomIntegerinRange 0 1))
              ;;[1 1 1] TARGET 3
              (AI|AIMoveTo self "0, 0, 0" (Variables|Default|GetTargetPoint3) 5.0 false :!label _label_3
                (:OnSuccess
                  (Utilities|FlowControl|Delay (Math|Random|RandomFloatinRange 1.0 3.0))
                  (CallFunction|Patrol)
                  ;;[1 0.2969 0.2969] If rng = 0 go to target 2, if = 1 move to 1
                  (if (== (Variables|Default|Get0) (Math|Random|RandomIntegerinRange 0 1))
                    (goto _label_2)
                    (else
                      (goto _label)))))
              (else
                (goto _label)))))
        (else
          (goto _label_3))))))

(event Custom|ResetAI
  ;[1 1 1] Reset pawn sensing
  (Class|PawnSensingComponent|SetSensingUpdatesEnabled (Variables|Default|GetPawnSensing) false)
  (switch Utilities|FlowControl|Switch|SwitchonE_AI_State (Variables|Default|GetAIState)
    (:NewEnumerator2
      (CallFunction|MovetoRandomLocation))
    (:NewEnumerator3
      (CallFunction|ChasePlayer))
    (:NewEnumerator4
      (CallFunction|Patrol))))

(event EventBeginPlay
  ;[1 1 1] Reset pawn sensing
  (bind _asfirst_person_character (Utilities|Casting|CastToFirstPersonCharacter (Game|GetPlayerCharacter 0)))
  (EventDispatchers|AssignPlayerDied _asfirst_person_character (delegate Custom|ResetAI))
  ;[1 1 1] Start state
  (switch Utilities|FlowControl|Switch|SwitchonE_AI_State (Variables|Default|GetAIState)
    (:NewEnumerator2
      (CallFunction|MovetoRandomLocation))
    (:NewEnumerator3
      (CallFunction|ChasePlayer))
    (:NewEnumerator4
      (CallFunction|Patrol))))

(fn ConstructionScript)